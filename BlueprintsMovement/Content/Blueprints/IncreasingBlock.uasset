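; IncreasingBlock is a block actor that grows each time another actor begins overlapping it.
; On BeginPlay it caches a scale step from its starting scale times SizeMultiplier.
; Each overlap adds that fixed step to the current scale, so growth is linear with no cap, then passes the event to the parent class's overlap handler.
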(event EventBeginPlay
  (Variables|Default|SetScaleDiff (* (Transformation|GetActorScale3D) (Variables|Default|GetSizeMultiplier))))

(event Collision|EventActorBeginOverlap
  (params (OtherActor :type Actor%20Object%20Reference))
  (Transformation|SetActorScale3D (+ (Transformation|GetActorScale3D) (Variables|Default|GetScaleDiff)))
  (|CallParentFunction OtherActor))

(fn ConstructionScript
  (|CallParentFunction))