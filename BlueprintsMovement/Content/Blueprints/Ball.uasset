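; Ball actor that bounces around in 2D, starting in a random direction at a clamped initial speed.
; Tick moves it with a swept world offset of Direction times Speed, without delta-time scaling.
; On a blocking hit it reflects Direction off the surface normal, then speeds up if the other object's name contains "Ball" and slows down otherwise, through the ChangeSpeed and ClampSpeed helpers.
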(event EventTick
  (params (DeltaSeconds :type Float%20%28single-precision%29))
  (Transformation|AddActorWorldOffset (* (Variables|Default|GetDirection) (Variables|Default|GetSpeed)) true))

(event EventBeginPlay
  (Variables|Default|SetDirection (Class|KismetMathLibrary|VectorNormal2D (Math|Random|RandomUnitVector) 0.0001))
  (Variables|Default|SetInitialSpeed (Utilities|ClampSpeed (Variables|Default|GetInitialSpeed)))
  (Variables|Default|SetSpeed (Variables|Default|GetInitialSpeed)))

(event Collision|EventHit
  (params (MyComp :type Primitive%20Component%20Object%20Reference) (Other :type Actor%20Object%20Reference) (OtherComp :type Primitive%20Component%20Object%20Reference) (bSelfMoved :type Boolean) (HitLocation :type Vector :default "0, 0, 0") (HitNormal :type Vector :default "0, 0, 0") (NormalImpulse :type Vector :default "0, 0, 0") (Hit :type Hit%20Result%20Structure%20%28by%20ref%29))
  (bind (_bblockinghit _binitialoverlap _time _distance _location _impactpoint _normal) (Collision|BreakHitResult Hit))
  (if _bblockinghit
    (Variables|Default|SetDirection (Class|KismetMathLibrary|VectorNormal2D (Math|Vector|GetReflectionVector (Variables|Default|GetDirection) _normal) 0.0001))
    (CallFunction|ChangeSpeed (Utilities|String|Contains (Utilities|GetObjectName Other) "Ball"))))

(fn ConstructionScript)

(fn ChangeSpeed
  (params (Increase :type Boolean))
  (if Increase
    (Variables|Default|SetSpeed (Utilities|ClampSpeed (+ (Variables|Default|GetSpeed) (Utilities|GetSpeedDifference))))
    (else
      (Variables|Default|SetSpeed (Utilities|ClampSpeed (- (Variables|Default|GetSpeed) (Utilities|GetSpeedDifference)))))))